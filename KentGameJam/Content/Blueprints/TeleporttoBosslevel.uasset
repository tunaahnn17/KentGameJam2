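; Trigger actor that teleports the player to the final boss level.
; When the player character enters its Box overlap volume, it shows two text widgets (WBP_YAZI4, then WBP_YAZI5) one second apart.
; After another one-second delay it opens LVL_Final_Boss by name; the widgets are only added, never explicitly removed.
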(event `self.Box.OnComponentBeginOverlap`
  (params (OverlappedComponent :type "PrimitiveComponent Object Reference") (OtherActor :type "Actor Object Reference") (OtherComp :type "PrimitiveComponent Object Reference") (OtherBodyIndex :type Integer) (bFromSweep :type Boolean) (SweepResult :type "HitResult Structure (by ref)"))
  (bind _returnvalue (`GameplayStatics.GetPlayerController` 0))
  (if (== (`GameplayStatics.GetPlayerCharacter` 0) OtherActor)
    (bind _returnvalue_2 (`|CreateWidget` "/Game/Widgets/WBP_YAZI4.WBP_YAZI4_C" _returnvalue))
    (`UserWidget.AddToViewport` _returnvalue_2 0)
    (`KismetSystemLibrary.Delay` 1.0)
    (bind _returnvalue_3 (`|CreateWidget` "/Game/Widgets/WBP_YAZI5.WBP_YAZI5_C" _returnvalue))
    (`UserWidget.AddToViewport` _returnvalue_3 0)
    (`KismetSystemLibrary.Delay` 1.0)
    (`GameplayStatics.OpenLevel` "LVL_Final_Boss")))

(fn `UserConstructionScript`)