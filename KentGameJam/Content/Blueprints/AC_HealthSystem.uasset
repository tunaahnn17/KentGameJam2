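; AC_HealthSystem is a health component that tracks current health (MevcutCan) against a maximum and calls the KarakterDead dispatcher at zero.
; BeginPlay fills health and binds HasarYedikOglim to the owner's OnTakeAnyDamage.
; The clamped health update and death check run in BeginPlay right after binding, while the damage handler itself is empty.
; The update computes Damage minus current health, rather than health minus Damage.
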(event `self.ReceiveBeginPlay`
  (set `self.Mevcut Can` (`self.Maksimum Can`))
  (add `Actor.OnTakeAnyDamage` (`self.GetOwner`) (delegate `HasarYedikOglim`))
  (set `self.Mevcut Can` (`KismetMathLibrary.FTrunc` (`KismetMathLibrary.FClamp` (- (stale `HasarYedikOglim` Damage) (`self.Mevcut Can`)) 0.0 (`KismetMathLibrary.Conv_IntToDouble` (`self.Maksimum Can`)))))
  (if (<= (`self.Mevcut Can`) 0)
    (`self.KarakterDead`)))

(event `HasarYedikOglim`
  (params (DamagedActor :type "Actor Object Reference") (Damage :type "Float (single-precision)") (DamageType :type "DamageType Object Reference") (InstigatedBy :type "Controller Object Reference") (DamageCauser :type "Actor Object Reference")))