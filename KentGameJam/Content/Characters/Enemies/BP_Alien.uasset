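; BP_Alien is an enemy that chases and attacks the player and can be killed by damage.
; PawnSensing sightings trigger an AI move to the player, and on success it plays a sped-up attack montage and applies fixed damage to the cached player character.
; Incoming damage lowers Health and updates the health bar widget, and the actor is destroyed when Health runs out.
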(event `self.ReceiveAnyDamage`
  (params (Damage :type "Float (single-precision)") (DamageType :type "DamageType Object Reference") (InstigatedBy :type "Controller Object Reference") (DamageCauser :type "Actor Object Reference"))
  ; Enemy Damage eating
  (bind _output_get (set `self.Health` (- (`self.Health`) Damage)))
  (bind _aswbp_enemy_health_bar (cast `/Game/Widgets/WBP_EnemyHealthBar` (`WidgetComponent.GetUserWidgetObject` (`self.Widget`))))
  (`ProgressBar.SetPercent` (`/Game/Widgets/WBP_EnemyHealthBar.EnemyHealthBar` _aswbp_enemy_health_bar) (/ _output_get 100.0))
  (if (<= _output_get 0.0)
    (`self.K2_DestroyActor`)))

(event `self.ReceiveBeginPlay`
  (bind _asbp_third_person_character (cast `/Game/ThirdPerson/Blueprints/BP_ThirdPersonCharacter` (`GameplayStatics.GetPlayerCharacter` 0)))
  (set `self.Character` _asbp_third_person_character))

(event `Follow Player`
  (`|AIMoveTo` self (0.0 0.0 0.0) (`GameplayStatics.GetPlayerCharacter` 0)
    (:`OnSuccess`
      (`self.PlayAnimMontage` "/Game/Characters/Mannequins/Anims/Unarmed/Attack/MM_Attack_02_Montage.MM_Attack_02_Montage" 3.0)
      (`GameplayStatics.ApplyDamage` (`self.Character`) 10.0))))

(event `self.PawnSensing.OnSeePawn`
  (params (Pawn :type "Pawn Object Reference"))
  (`self.Follow Player`))

(fn `UserConstructionScript`)