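; BP_Boss1 is a boss enemy that faces the player, fires projectiles and dies when its health runs out.
; Tick turns its yaw toward the player character cached on BeginPlay.
; Pawn sensing triggers a delayed attack that spawns BP_Projectile at the muzzle transform.
; Any damage lowers Health and updates the widget health bar, assuming a 100-point maximum, then destroys the actor at zero.
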(event `self.ReceiveAnyDamage`
  (params (Damage :type "Float (single-precision)") (DamageType :type "DamageType Object Reference") (InstigatedBy :type "Controller Object Reference") (DamageCauser :type "Actor Object Reference"))
  ; Enemy Damage eating
  (bind _output_get (set `self.Health` (- (`self.Health`) Damage)))
  (bind _aswbp_enemy_health_bar (cast `/Game/Widgets/WBP_EnemyHealthBar` (`WidgetComponent.GetUserWidgetObject` (`self.Widget`))))
  (`ProgressBar.SetPercent` (`/Game/Widgets/WBP_EnemyHealthBar.EnemyHealthBar` _aswbp_enemy_health_bar) (/ _output_get 100.0))
  (if (<= _output_get 0.0)
    (`self.K2_DestroyActor`)))

(event `ThrowProjectile`
  (`|SpawnActorFromClass` "/Game/Blueprints/BP_Projectile.BP_Projectile_C" (`SceneComponent.K2_GetComponentToWorld` (`self.MuzzleLocation`)) "Undefined" "MultiplyWithRoot" null null))

(event `self.ReceiveBeginPlay`
  (bind _asbp_third_person_character (cast `/Game/ThirdPerson/Blueprints/BP_ThirdPersonCharacter` (`GameplayStatics.GetPlayerCharacter` 0)))
  (set `self.character` _asbp_third_person_character))

(event `self.PawnSensing.OnSeePawn`
  (params (Pawn :type "Pawn Object Reference"))
  (`self.StartAttacking`))

(event `StartAttacking`
  (`KismetSystemLibrary.Delay` 0.6)
  (`self.ThrowProjectile`)
  (`KismetSystemLibrary.Delay` 0.2))

(event `self.ReceiveTick`
  (params (DeltaSeconds :type "Float (single-precision)"))
  (bind (_returnvalue_roll _returnvalue_pitch _returnvalue_yaw) (`KismetMathLibrary.BreakRotator` (`KismetMathLibrary.FindLookAtRotation` (`self.K2_GetActorLocation`) (`self.K2_GetActorLocation` (`self.character`)))))
  (`self.K2_SetActorRotation` (`KismetMathLibrary.MakeRotator` 0.0 0.0 _returnvalue_yaw)))

(fn `UserConstructionScript`)