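; BP_Enemy1 is an enemy that chases the player and attacks on reaching them.
; Pawn sensing triggers an AI move to the player, whose success calls a montage play and applies damage.
; Tick keeps its yaw turned toward the cached player character.
; Incoming damage lowers Health and casts the health bar widget, but the bar update and zero-health destroy logic are left unconnected.
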(event `self.ReceiveAnyDamage`
  (params (Damage :type "Float (single-precision)") (DamageType :type "DamageType Object Reference") (InstigatedBy :type "Controller Object Reference") (DamageCauser :type "Actor Object Reference"))
  (bind _output_get (set `self.health` (- (`self.health`) Damage)))
  (cast `/Game/Widget/WBP_HealthBar` (`WidgetComponent.GetUserWidgetObject` (`self.Widget`))))

(event `self.ReceiveBeginPlay`
  (bind _asbp_third_person_character (cast `/Game/ThirdPerson/Blueprints/BP_ThirdPersonCharacter` (`GameplayStatics.GetPlayerCharacter` 0)))
  (set `self.character` _asbp_third_person_character))

(event `Follow Player`
  (`|AIMoveTo` self (0.0 0.0 0.0) (`GameplayStatics.GetPlayerCharacter` 0)
    (:`OnSuccess`
      ; Dikkat
      (`self.PlayAnimMontage` null) ; karaktere göre animasyonu seçin
      (`GameplayStatics.ApplyDamage` (`self.character`)))))

(event `self.PawnSensing.OnSeePawn`
  (params (Pawn :type "Pawn Object Reference"))
  (`self.Follow Player`))

(event `self.ReceiveTick`
  (params (DeltaSeconds :type "Float (single-precision)"))
  (bind (_returnvalue_roll _returnvalue_pitch _returnvalue_yaw) (`KismetMathLibrary.BreakRotator` (`KismetMathLibrary.FindLookAtRotation` (`self.K2_GetActorLocation`) (`self.K2_GetActorLocation` (`self.character`)))))
  (`self.K2_SetActorRotation` (`KismetMathLibrary.MakeRotator` 0.0 0.0 _returnvalue_yaw)))

(fn `UserConstructionScript`)